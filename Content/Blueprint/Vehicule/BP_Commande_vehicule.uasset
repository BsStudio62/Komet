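; BP_Commande_vehicule is a trigger actor, named as a vehicle control, that registers itself as the interaction target of characters standing in its Box.
; Overlap begin and end run only with authority, setting and then clearing that reference.
; BP_ThirdPersonCharacter also has god mode enabled while inside, while the fallback cast to BP_Proto_ThirdPersonCharacter only sets the Interaction variable.
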(event OnComponentBeginOverlap(Box)
  (params (OverlappedComponent :type Primitive%20Component%20Object%20Reference) (OtherActor :type Actor%20Object%20Reference) (OtherComp :type Primitive%20Component%20Object%20Reference) (OtherBodyIndex :type Integer) (bFromSweep :type Boolean) (SweepResult :type Hit%20Result%20Structure%20%28by%20ref%29))
  (Networking|SwitchHasAuthority
    (:Authority
      (bind _asbp_third_person_character (Utilities|Casting|CastToBP_ThirdPersonCharacter OtherActor)
        (:then
          (Class|KometCharacter|SetInteraction _asbp_third_person_character self)
          (Class|KometCharacter|SetGodMod _asbp_third_person_character true))
        (:CastFailed
          (bind _asbp_proto_third_person_character (Utilities|Casting|CastToBP_Proto_ThirdPersonCharacter OtherActor))
          (Variables|/Game/Characters/BP_Proto_ThirdPersonCharacter.BP_Proto_ThirdPersonCharacter_C|SetInteraction _asbp_proto_third_person_character self))))))

(event OnComponentEndOverlap(Box)
  (params (OverlappedComponent :type Primitive%20Component%20Object%20Reference) (OtherActor :type Actor%20Object%20Reference) (OtherComp :type Primitive%20Component%20Object%20Reference) (OtherBodyIndex :type Integer))
  (Networking|SwitchHasAuthority
    (:Authority
      (bind _asbp_third_person_character (Utilities|Casting|CastToBP_ThirdPersonCharacter OtherActor)
        (:then
          (Class|KometCharacter|SetInteraction _asbp_third_person_character)
          (Class|KometCharacter|SetGodMod _asbp_third_person_character false))
        (:CastFailed
          (bind _asbp_proto_third_person_character (Utilities|Casting|CastToBP_Proto_ThirdPersonCharacter OtherActor))
          (Variables|/Game/Characters/BP_Proto_ThirdPersonCharacter.BP_Proto_ThirdPersonCharacter_C|SetInteraction _asbp_proto_third_person_character 0))))))

(fn ConstructionScript)