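; BP_Proto_Grenade is a prototype grenade actor that explodes after a timed delay.
; On BeginPlay, only the authority waits DelayExplosion, then applies radial damage with falloff between an inner and outer radius.
; It then calls an event that spawns the explosion particles and sound, optionally draws both radii as debug spheres when IsDebug is set, and destroys itself.
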(event Custom|Play%20Sound%20&%20FX
  ;[1 1 1] Play FX and Sound
  (Effects|SpawnEmitteratLocation "/Game/Template/StarterContent/Particles/P_Explosion.P_Explosion" (Transformation|GetActorLocation) "0, 0, 0" "2.000000,2.000000,2.000000")
  (Audio|PlaySoundatLocation "/Game/Template/StarterContent/Audio/Explosion_Cue.Explosion_Cue" (Transformation|GetActorLocation) "0, 0, 0" 1.0 1.0 0.0 0 0 0 0))

(event EventBeginPlay
  (bind _returnvalue (Transformation|GetActorLocation))
  (Networking|SwitchHasAuthority
    (:Authority
      (Utilities|FlowControl|Delay (Variables|Default|GetDelay%20Explosion))
      (Class|GameplayStatics|ApplyRadialDamagewithFalloff 1e+02 1e+01 (Transformation|GetActorLocation) (Variables|Default|GetDamage%20Inner%20Radius) (Variables|Default|GetDamage%20Outer%20Radius) 1.0 0 0 self 0 "ECC_Pawn")
      (CallFunction|PlaySound&FX)
      (if (Variables|Default|GetbIsDebug)
        ;[1 1 1] Debug System
        (Rendering|Debug|DrawDebugSphere _returnvalue (Variables|Default|GetDamage%20Inner%20Radius) 12 "(R=1.000000,G=0.000000,B=0.670606,A=1.000000)" 5.0 1.0)
        (Rendering|Debug|DrawDebugSphere _returnvalue (Variables|Default|GetDamage%20Outer%20Radius) 12 "(R=0.000000,G=1.000000,B=0.985854,A=1.000000)" 5.0 1.0))
      (Actor|DestroyActor))))

(fn ConstructionScript)