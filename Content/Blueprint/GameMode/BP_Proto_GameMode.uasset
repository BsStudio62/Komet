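; Prototype GameMode that spawns and possesses a third-person character for each player who logs in.
; On PostLogin it stores the controller in an array, spawns the character at a player start, and uses the array index to select one of three colors.
; A respawn loop that restarts players lacking a valid pawn is present but disconnected from Tick, so it never runs.
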(event EventTick
  (params (DeltaSeconds :type Float%20%28single-precision%29))
  ;[1 1 1] Respawn Systeme
)

(event EventPostLogin
  (params (NewPlayer :type Player%20Controller%20Object%20Reference))
  (bind _returnvalue (Utilities|Array|Add (Variables|Default|GetNew%20Player) NewPlayer))
  (bind _returnvalue_2 (Game|SpawnActorfromClass "/Game/Characters/BP_Proto_ThirdPersonCharacter.BP_Proto_ThirdPersonCharacter_C" (Transformation|GetActorTransform (Class|GameModeBase|FindPlayerStart NewPlayer)) "Undefined" "MultiplyWithRoot" 0 0))
  (Default|SetColor _returnvalue_2 (Utilities|Select :Index _returnvalue :Option%200 "(R=0.000000,G=1.000000,B=0.138169,A=1.000000)" :Option%201 "(R=1.000000,G=0.000000,B=0.000000,A=1.000000)" :Option%202 "(R=0.000000,G=1.000000,B=0.950529,A=1.000000)"))
  (Pawn|Possess NewPlayer _returnvalue_2))

(fn ConstructionScript)