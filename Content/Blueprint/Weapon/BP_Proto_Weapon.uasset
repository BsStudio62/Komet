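; Prototype hitscan weapon Blueprint that damages Pawns hit by a line trace.
; Fire branches on authority into two custom events that share the same trace logic, with the remote event also calling the authority one.
; The trace runs from the Muzzle socket along the owner's view rotation, ignores the owner and draws debug lines.
; Damage to a hit Pawn is applied only with authority.
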(event Custom|Fire
  (Networking|SwitchHasAuthority
    (:Authority
      (CallFunction|CustomEvent0))
    (:Remote
      (CallFunction|CustomEvent))))

(event Custom|CustomEvent
  (bind _skeletalmesh (Variables|Default|GetSkeletalMesh))
  (bind _returnvalue (Transformation|GetSocketLocation _skeletalmesh "Muzzle"))
  (CallFunction|CustomEvent0)
  (bind (_outhit _returnvalue_2) (Collision|LineTraceByChannel _returnvalue (+ _returnvalue (* (Math|Rotator|GetRotationXVector (.OutRotation (Actor|GetActorEyesViewPoint (Components|GetOwner)))) 1e+04)) "TraceTypeQuery1" false (Utilities|Array|MakeArray (Components|GetOwner)) "ForDuration"))
  (if _returnvalue_2
    (Utilities|Casting|CastToPawn (.HitActor (Collision|BreakHitResult _outhit)))
    (Networking|SwitchHasAuthority
      (:Authority
        (Game|Damage|ApplyDamage (.HitActor (Collision|BreakHitResult _outhit)) 1e+02 0 self)))))

(event Custom|CustomEvent_0
  (bind _skeletalmesh (Variables|Default|GetSkeletalMesh))
  (bind _returnvalue (Transformation|GetSocketLocation _skeletalmesh "Muzzle"))
  (bind (_outhit _returnvalue_2) (Collision|LineTraceByChannel _returnvalue (+ _returnvalue (* (Math|Rotator|GetRotationXVector (.OutRotation (Actor|GetActorEyesViewPoint (Components|GetOwner)))) 1e+04)) "TraceTypeQuery1" false (Utilities|Array|MakeArray (Components|GetOwner)) "ForDuration"))
  (if _returnvalue_2
    (Utilities|Casting|CastToPawn (.HitActor (Collision|BreakHitResult _outhit)))
    (Networking|SwitchHasAuthority
      (:Authority
        (Game|Damage|ApplyDamage (.HitActor (Collision|BreakHitResult _outhit)) 1e+02 0 self)))))

(fn ConstructionScript)